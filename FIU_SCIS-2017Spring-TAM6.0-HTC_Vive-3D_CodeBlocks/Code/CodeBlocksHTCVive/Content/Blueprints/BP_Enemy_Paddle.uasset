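; BP_Enemy_Paddle is an AI-controlled paddle that chases the ball along the X axis.
; On BeginPlay it sets its speed from the Easy, Normal or Hard difficulty string in CodeBlocksGameInstance.
; Each Tick it finds every BP_Ball and applies a physics impulse toward each, using the clamped X offset scaled by speed.
; Past either map limit, it instead snaps just inside at zero Y and Z and clears velocity.
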(event EventBeginPlay
  ;[1 1 1] Set AI Difficulty
  (bind _ascode_blocks_game_instance (Utilities|Casting|CastToCodeBlocksGameInstance (Game|GetGameInstance)))
  (if (Utilities|Enum|Equal(Enum) (Variables|/Game/Blueprints/CodeBlocksGameInstance.CodeBlocksGameInstance_C|GetAIDifficulty _ascode_blocks_game_instance) "Easy")
    (Variables|Default|SetAI_Paddle_Speed 4e+03)
    (elif (Utilities|Enum|Equal(Enum) (Variables|/Game/Blueprints/CodeBlocksGameInstance.CodeBlocksGameInstance_C|GetAIDifficulty _ascode_blocks_game_instance) "Normal")
      (Variables|Default|SetAI_Paddle_Speed 8e+03)
      (elif (Utilities|Enum|Equal(Enum) (Variables|/Game/Blueprints/CodeBlocksGameInstance.CodeBlocksGameInstance_C|GetAIDifficulty _ascode_blocks_game_instance) "Hard")
        (Variables|Default|SetAI_Paddle_Speed 1.2e+04)))))

(event Collision|EventActorBeginOverlap
  (params (OtherActor :type Actor%20Object%20Reference)))

(event EventTick
  (params (DeltaSeconds :type Float%20%28single-precision%29))
  ;[1 1 1] Get Ball
  (bind _outactors (Actor|GetAllActorsOfClass "/Game/Blueprints/BP_Ball.BP_Ball_C"))
  (for _array_element _outactors
    (bind _asbp_ball (Utilities|Casting|CastToBP_Ball _array_element))
    ;[1 1 1] Keep Enemy Paddle From Going Above The Map
    (if (> (.X (Math|Vector|BreakVector (Transformation|GetActorLocation))) 1.5e+03)
      (Transformation|SetActorLocation (Math|Vector|MakeVector 1499.0 0.0 0.0) false false)
      (Physics|SetPhysicsLinearVelocity (Variables|Default|GetStaticMesh) "0, 0, 0" false "None")
      (else
        ;[1 1 1] Keep Enemy Paddle From Going Below The Map
        (if (< (.X (Math|Vector|BreakVector (Transformation|GetActorLocation))) -1.5e+03)
          (Transformation|SetActorLocation (Math|Vector|MakeVector -1499.0 0.0 0.0) false false)
          (Physics|SetPhysicsLinearVelocity (Variables|Default|GetStaticMesh) "0, 0, 0" false "None")
          (else
            ;[1 1 1] Move Enemy Paddle Towards Ball
            (Physics|AddImpulse (Variables|Default|GetStaticMesh) (* (Math|Vector|MakeVector (Math|Float|Clamp(Float) (- (.X (Math|Vector|BreakVector (Transformation|GetActorLocation _asbp_ball))) (.X (Math|Vector|BreakVector (Transformation|GetActorLocation)))) -1e+01 1e+01) 0.0 0.0) (Variables|Default|GetAI_Paddle_Speed)) "None" false)))))))

(fn ConstructionScript)