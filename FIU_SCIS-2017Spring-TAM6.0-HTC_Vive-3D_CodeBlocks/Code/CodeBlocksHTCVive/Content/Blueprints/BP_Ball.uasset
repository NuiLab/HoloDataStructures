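; Pong-style ball that drives movement, scoring and game over for one- and two-player matches.
; BeginPlay takes launch speed and score limit from CodeBlocksGameInstance.
; Overlaps flip physics velocity at paddles and boundaries, with random paddle deflection; goals recenter the ball at a fixed speed and update tagged TextRenderActor scores.
; At the limit, Tick stops the ball and, after a delay, opens P2_Main if BP_Paddle_Left exists, otherwise P1_Main.
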(event EventBeginPlay
  (bind _ascode_blocks_game_instance (Utilities|Casting|CastToCodeBlocksGameInstance (Game|GetGameInstance)))
  ;[1 1 1] Set Ball Velocity
  (if (Utilities|Enum|Equal(Enum) (Variables|/Game/Blueprints/CodeBlocksGameInstance.CodeBlocksGameInstance_C|GetBallSpeed _ascode_blocks_game_instance) "Slow")
    (Variables|Default|SetBallVelocity 1500)
    (Physics|SetPhysicsLinearVelocity (Variables|Default|GetStaticMesh) (Math|Vector|MakeVector 0.0 (Math|Conversions|ToFloat(Integer) (Variables|Default|GetBallVelocity)) 0.0) false "None" :!label _label)
    ;[1 1 1] Set Max Point Amount
    (if (> (Math|Conversions|ToInteger(Byte) (Variables|/Game/Blueprints/CodeBlocksGameInstance.CodeBlocksGameInstance_C|GetScoreLimit _ascode_blocks_game_instance)) 0)
      (Variables|Default|SetMaxPoints (Variables|/Game/Blueprints/CodeBlocksGameInstance.CodeBlocksGameInstance_C|GetScoreLimit _ascode_blocks_game_instance)))
    (elif (Utilities|Enum|Equal(Enum) (Variables|/Game/Blueprints/CodeBlocksGameInstance.CodeBlocksGameInstance_C|GetBallSpeed _ascode_blocks_game_instance) "Average")
      (Variables|Default|SetBallVelocity 2000)
      (goto _label)
      (elif (Utilities|Enum|Equal(Enum) (Variables|/Game/Blueprints/CodeBlocksGameInstance.CodeBlocksGameInstance_C|GetBallSpeed _ascode_blocks_game_instance) "Fast")
        (Variables|Default|SetBallVelocity 2500)
        (goto _label)))))

(event Collision|EventActorBeginOverlap
  (params (OtherActor :type Actor%20Object%20Reference))
  (bind _maxpoints (Variables|Default|GetMaxPoints))
  ;[1 1 1] Player 1 Hit Logic
  (Utilities|Casting|CastToBP_Paddle_Right OtherActor
    (:then
      (bind _returnvalue (Physics|GetPhysicsLinearVelocity (Variables|Default|GetStaticMesh) "None"))
      (bind _returnvalue_2 (Physics|GetPhysicsLinearVelocity (Variables|Default|GetStaticMesh) "None"))
      (Physics|SetPhysicsLinearVelocity (Variables|Default|GetStaticMesh) (Math|Vector|MakeVector (+ (.X (Math|Vector|BreakVector _returnvalue)) (Math|Random|RandomFloatinRange -1e+03 1e+03)) (* (.Y (Math|Vector|BreakVector _returnvalue_2)) -1.0) (.Z (Math|Vector|BreakVector _returnvalue_2))) false "None")
      (Audio|PlaySoundatLocation "/Game/Audio/S_ballCollision.S_ballCollision" "0, 0, 0"))
    (:CastFailed
      ;[1 1 1] Player 2 Hit Logic
      (bind _asbp_paddle_left (Utilities|Casting|CastToBP_Paddle_Left OtherActor)
        (:then
          (bind _returnvalue_3 (Physics|GetPhysicsLinearVelocity (Variables|/Game/Blueprints/BP_Paddle_Left.BP_Paddle_Left_C|GetStaticMesh _asbp_paddle_left) "None"))
          (bind _returnvalue_4 (Physics|GetPhysicsLinearVelocity (Variables|Default|GetStaticMesh) "None"))
          (Physics|SetPhysicsLinearVelocity (Variables|Default|GetStaticMesh) (Math|Vector|MakeVector (+ (.X (Math|Vector|BreakVector _returnvalue_3)) (Math|Random|RandomFloatinRange -1e+03 1e+03)) (* (.Y (Math|Vector|BreakVector _returnvalue_4)) -1.0) (.Z (Math|Vector|BreakVector _returnvalue_4))) false "None")
          (Audio|PlaySoundatLocation "/Game/Audio/S_ballCollision.S_ballCollision" "0, 0, 0"))
        (:CastFailed
          ;[1 1 1] Horizontal Boundary Hit Logic
          (Utilities|Casting|CastToBP_Horizontal_Boundary OtherActor
            (:then
              (bind _returnvalue_5 (Physics|GetPhysicsLinearVelocity (Variables|Default|GetStaticMesh) "None"))
              (Physics|SetPhysicsLinearVelocity (Variables|Default|GetStaticMesh) (Math|Vector|MakeVector (* (.X (Math|Vector|BreakVector _returnvalue_5)) -1.0) (.Y (Math|Vector|BreakVector _returnvalue_5)) (.Z (Math|Vector|BreakVector _returnvalue_5))) false "None")
              (Audio|PlaySoundatLocation "/Game/Audio/S_ballCollision.S_ballCollision" "0, 0, 0"))
            (:CastFailed
              ;[1 1 1] Goal Logic
              (Utilities|Casting|CastToBP_Left_Goal OtherActor
                (:then
                  (Transformation|SetActorLocation "0,0.000000, 0" false false)
                  (Physics|SetPhysicsLinearVelocity (Variables|Default|GetStaticMesh) "0,2000.000000, 0" false "None")
                  (Audio|PlaySoundatLocation "/Game/Audio/S_ballGoal.S_ballGoal" "0, 0, 0")
                  (Variables|Default|SetRPlayer_Score (+ (Variables|Default|GetRPlayer_Score) 1))
                  (bind _outactors (Actor|GetAllActorsOfClass "/Script/Engine.TextRenderActor"))
                  (for _array_element _outactors
                    (bind _astext_render_actor (Utilities|Casting|CastToTextRenderActor _array_element))
                    (if (Components|ComponentHasTag (Variables|/Script/Engine.TextRenderActor|GetTextRender _astext_render_actor) "R_Player_Score_Tag")
                      (Rendering|Components|TextRender|SetText (Variables|/Script/Engine.TextRenderActor|GetTextRender _astext_render_actor) (Utilities|Text|ToText(Integer) (Variables|Default|GetRPlayer_Score)))
                      (if (>= (Variables|Default|GetRPlayer_Score) (Math|Conversions|ToInteger(Byte) _maxpoints))
                        (Development|PrintString "Right Side Wins" true true "(R=0.000000,G=0.660000,B=1.000000,A=1.000000)" 3.0)
                        (Variables|Default|SetGameOver true)))))
                (:CastFailed
                  (Utilities|Casting|CastToBP_Right_Goal OtherActor
                    (:then
                      (Transformation|SetActorLocation "0,0.000000, 0" false false)
                      (Physics|SetPhysicsLinearVelocity (Variables|Default|GetStaticMesh) "0,-2000.000000, 0" false "None")
                      (Audio|PlaySoundatLocation "/Game/Audio/S_ballGoal.S_ballGoal" "0, 0, 0")
                      (Variables|Default|SetLPlayer_Score (+ (Variables|Default|GetLPlayer_Score) 1))
                      (bind _outactors_2 (Actor|GetAllActorsOfClass "/Script/Engine.TextRenderActor"))
                      (for _array_element_2 _outactors_2
                        (bind _astext_render_actor_2 (Utilities|Casting|CastToTextRenderActor _array_element_2))
                        (if (Components|ComponentHasTag (Variables|/Script/Engine.TextRenderActor|GetTextRender _astext_render_actor_2) "L_Player_Score_Tag")
                          (Rendering|Components|TextRender|SetText (Variables|/Script/Engine.TextRenderActor|GetTextRender _astext_render_actor_2) (Utilities|Text|ToText(Integer) (Variables|Default|GetLPlayer_Score)))
                          (if (>= (Variables|Default|GetLPlayer_Score) (Math|Conversions|ToInteger(Byte) _maxpoints))
                            (Development|PrintString "Left Side Wins" true true "(R=0.000000,G=0.660000,B=1.000000,A=1.000000)" 3.0)
                            (Variables|Default|SetGameOver true)))))
                    (:CastFailed
                      ;[1 1 1] Add Random X Amount to Enemy Paddle Hit
                      (bind _asbp_enemy_paddle (Utilities|Casting|CastToBP_Enemy_Paddle OtherActor))
                      (bind _returnvalue_6 (Physics|GetPhysicsLinearVelocity (Variables|/Game/Blueprints/BP_Enemy_Paddle.BP_Enemy_Paddle_C|GetStaticMesh _asbp_enemy_paddle) "None"))
                      (Audio|PlaySoundatLocation "/Game/Audio/S_ballCollision.S_ballCollision" "0, 0, 0")
                      (bind _returnvalue_7 (Physics|GetPhysicsLinearVelocity (Variables|Default|GetStaticMesh) "None"))
                      (Physics|SetPhysicsLinearVelocity (Variables|Default|GetStaticMesh) (Math|Vector|MakeVector (+ (.X (Math|Vector|BreakVector _returnvalue_6)) (Math|Random|RandomFloatinRange -5e+02 5e+02)) (* (.Y (Math|Vector|BreakVector _returnvalue_7)) -1.0) (.Z (Math|Vector|BreakVector _returnvalue_7))) false "None"))))))))))))

(event EventTick
  (params (DeltaSeconds :type Float%20%28single-precision%29))
  ;[1 1 1] Satrt Game After Game Over
  (if (Variables|Default|GetGameOver)
    (Physics|SetPhysicsLinearVelocity (Variables|Default|GetStaticMesh) "0, 0, 0" false "None")
    (Utilities|FlowControl|Delay 3.0)
    (bind _outactors (Actor|GetAllActorsOfClass "/Game/Blueprints/BP_Paddle_Left.BP_Paddle_Left_C"))
    (if (> (Utilities|Array|Length _outactors) 0)
      (Game|OpenLevel(byName) "P2_Main")
      (else
        (Game|OpenLevel(byName) "P1_Main")))))

(fn ConstructionScript)