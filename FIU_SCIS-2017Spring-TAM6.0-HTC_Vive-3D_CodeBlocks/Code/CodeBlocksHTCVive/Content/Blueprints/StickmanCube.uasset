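; StickmanCube is a cube actor that switches between a raised position and its origin in response to event dispatchers.
; On BeginPlay it binds custom events to the MovingUp and MoveToOrigin dispatchers.
; Those events snap the cube to a fixed height at its original X and Y, or back to its stored original location, without sweep or interpolation.
; The file does not set those stored coordinates.
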(event Custom|MovingUpEvent
  (CallFunction|MoveUp))

(event Custom|MoveToOriginEvent
  (CallFunction|MovetoOrigin))

(event EventBeginPlay
  (EventDispatchers|BindEventtoMovingUpDispatcher (delegate Custom|MovingUpEvent))
  (EventDispatchers|BindEventtoMovetoOriginDispatcher (delegate Custom|MoveToOriginEvent)))

(event Collision|EventActorBeginOverlap
  (params (OtherActor :type Actor%20Object%20Reference)))

(event EventTick
  (params (DeltaSeconds :type Float%20%28single-precision%29)))

(fn ConstructionScript)

(fn MoveUp
  (Transformation|SetActorLocation (Math|Vector|MakeVector (Variables|Default|GetOriginal%20X) (Variables|Default|GetOriginal%20Y) 2.1e+02) false false))

(fn MovetoOrigin
  (Transformation|SetActorLocation (Math|Vector|MakeVector (Variables|Default|GetOriginal%20X) (Variables|Default|GetOriginal%20Y) (Variables|Default|GetOriginal%20Z)) false false))