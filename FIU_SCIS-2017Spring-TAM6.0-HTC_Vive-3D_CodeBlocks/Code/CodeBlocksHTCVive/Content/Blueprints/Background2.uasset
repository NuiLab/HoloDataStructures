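; Background2 is a background mesh actor that applies the background choice stored in CodeBlocksGameInstance.
; On BeginPlay it compares the Background string, hiding the mesh for Black or swapping its first material for Ocean, Pine or Grass.
; Each instance applies the change to every Background2 actor found through GetAllActorsOfClass, not just itself, and other values leave the meshes unchanged.
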(event EventBeginPlay
  (bind _ascode_blocks_game_instance (Utilities|Casting|CastToCodeBlocksGameInstance (Game|GetGameInstance)))
  (if (Utilities|Enum|Equal(Enum) (Variables|/Game/Blueprints/CodeBlocksGameInstance.CodeBlocksGameInstance_C|GetBackground _ascode_blocks_game_instance) "Black")
    (bind _outactors (Actor|GetAllActorsOfClass "Background2_C"))
    (for _array_element _outactors
      (bind _asbackground_2 (Utilities|Casting|CastToBackground2 _array_element))
      (Rendering|SetVisibility (Variables|Background2_C|GetStaticMesh _asbackground_2) false false))
    (elif (Utilities|Enum|Equal(Enum) (Variables|/Game/Blueprints/CodeBlocksGameInstance.CodeBlocksGameInstance_C|GetBackground _ascode_blocks_game_instance) "Ocean")
      (bind _outactors_2 (Actor|GetAllActorsOfClass "Background2_C"))
      (for _array_element_2 _outactors_2
        (bind _asbackground_2_2 (Utilities|Casting|CastToBackground2 _array_element_2))
        (Rendering|Material|SetMaterial (Variables|Background2_C|GetStaticMesh _asbackground_2_2) 0 "/Game/StarterContent/Materials/M_Water_Ocean.M_Water_Ocean"))
      (elif (Utilities|Enum|Equal(Enum) (Variables|/Game/Blueprints/CodeBlocksGameInstance.CodeBlocksGameInstance_C|GetBackground _ascode_blocks_game_instance) "Pine")
        (bind _outactors_3 (Actor|GetAllActorsOfClass "Background2_C"))
        (for _array_element_3 _outactors_3
          (bind _asbackground_2_3 (Utilities|Casting|CastToBackground2 _array_element_3))
          (Rendering|Material|SetMaterial (Variables|Background2_C|GetStaticMesh _asbackground_2_3) 0 "/Game/StarterContent/Materials/M_Wood_Pine.M_Wood_Pine"))
        (elif (Utilities|Enum|Equal(Enum) (Variables|/Game/Blueprints/CodeBlocksGameInstance.CodeBlocksGameInstance_C|GetBackground _ascode_blocks_game_instance) "Grass")
          (bind _outactors_4 (Actor|GetAllActorsOfClass "Background2_C"))
          (for _array_element_4 _outactors_4
            (bind _asbackground_2_4 (Utilities|Casting|CastToBackground2 _array_element_4))
            (Rendering|Material|SetMaterial (Variables|Background2_C|GetStaticMesh _asbackground_2_4) 0 "/Game/StarterContent/Materials/M_Ground_Grass.M_Ground_Grass")))))))

(event Collision|EventActorBeginOverlap
  (params (OtherActor :type Actor%20Object%20Reference)))

(event EventTick
  (params (DeltaSeconds :type Float%20%28single-precision%29)))

(fn ConstructionScript)