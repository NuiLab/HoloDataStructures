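; BP_Paddle_Left is the left paddle actor, driven by the Player2MoveUp input axis.
; Each tick it applies a large physics force to its static mesh along world X, scaled by the axis value.
; When X passes either symmetric limit, it instead snaps just inside that bound without sweep, resetting Y and Z to zero.
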(event Collision|EventActorBeginOverlap
  (params (OtherActor :type Actor%20Object%20Reference)))

(event EventTick
  (params (DeltaSeconds :type Float%20%28single-precision%29))
  (if (> (.X (Math|Vector|BreakVector (Transformation|GetActorLocation))) 1.5e+03)
    (Transformation|SetActorLocation (Math|Vector|MakeVector 1499.0 0.0 0.0) false false)
    (elif (< (.X (Math|Vector|BreakVector (Transformation|GetActorLocation))) -1.5e+03)
      (Transformation|SetActorLocation (Math|Vector|MakeVector -1499.0 0.0 0.0) false false)
      (else
        (Physics|AddForce (Variables|Default|GetStaticMesh) (Math|Vector|MakeVector (* (Input|AxisValues|GetPlayer2MoveUp) 9e+06) 0.0 0.0) "None" false)))))

(fn ConstructionScript)